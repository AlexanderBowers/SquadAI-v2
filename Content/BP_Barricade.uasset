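; BP_Barricade is a barricade that a squad commando can be ordered to blow up.
; CheckAssignedMember assigns an available member from SquadPlayerController through its blackboard, or, if one is already assigned, detonates the bomb and destroys the barricade.
; When the assigned commando overlaps, it spawns BP_Bomb at BombLocation and a short timer releases the member's priority command.
; ResetAssignedMember only prints debug text when no member is valid.
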(event `self.ReceiveActorBeginOverlap`
  (params (OtherActor :type "Actor Object Reference"))
  (bind _asbp_commando (cast `/Game/AI_Portfolio_Migration/BP_Commando` OtherActor)
    (:`then`
      (if (== _asbp_commando (`Controller.K2_GetPawn` (`self.AssignedSquadMember`)))
        (bind _returnvalue (`|SpawnActorFromClass` "/Game/BP_Bomb.BP_Bomb_C" (`SceneComponent.K2_GetComponentToWorld` (`self.BombLocation`)) "Undefined" "OverrideRootScale" null null))
        (`KismetSystemLibrary.K2_SetTimer` null "SetBombTimer" 2.5)
        (else
          (`KismetSystemLibrary.PrintText` "Failed :("))))
    (:`CastFailed`
      (`KismetSystemLibrary.PrintText` "Cast failed!!"))))

(event `SquadInterface.CheckAssignedMember`
  (params (CommandPoint :type "CommandPoint Structure"))
  (bind (_location _type _owneractor) (break `CommandPoint` CommandPoint))
  (`/Engine/EditorBlueprintResources/StandardMacros.IsValid` (`self.AssignedSquadMember`)
    (:`Is Valid`
      (`KismetSystemLibrary.PrintText` "TIME TO BLOWWWWW")
      (`/Game/BP_Bomb.Explode` (stale `self.ReceiveActorBeginOverlap` _returnvalue))
      (`self.K2_DestroyActor`))
    (:`Is Not Valid`
      (bind _assquad_player_controller (cast `SquadPlayerController` (`GameplayStatics.GetPlayerController` 0)))
      (bind _returnvalue (`SquadPlayerController.GetAvailableMember` _assquad_player_controller (make `CommandPoint` (`SceneComponent.K2_GetComponentLocation` (`self.BombLocation`)) _type _owneractor)))
      (bind _returnvalue_2 (`AIBlueprintHelperLibrary.GetBlackboard` _returnvalue))
      (`BlackboardComponent.SetValueAsObject` _returnvalue_2 "AssignedPosition" self)
      (`BlackboardComponent.SetValueAsBool` _returnvalue_2 "bIsAssigned" true)
      (set `self.AssignedSquadMember` _returnvalue))))

(event `SquadInterface.ResetAssignedMember`
  (`/Engine/EditorBlueprintResources/StandardMacros.IsValid` (`self.AssignedSquadMember`)
    (:`Is Not Valid`
      (`KismetSystemLibrary.PrintString` "Reset Called but not valid."))))

(event `SetBombTimer`
  (`SquadAIController.ResetPriorityCommand` (`self.AssignedSquadMember`)))

(fn `UserConstructionScript`)