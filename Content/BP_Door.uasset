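; BP_Door is a door actor that serves as a command target for the player's squad.
; On CheckAssignedMember, it asks BP_SquadPlayerController for three available members, passing command points at the BombLocation, Assist1 and Assist2 components.
; Each point keeps the incoming command's type and owner, and each returned member is stored as an assigned squad member.
; OpenDoor currently applies a zero local offset, so the door does not move.
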(event `SquadInterface.CheckAssignedMember`
  (params (CommandPoint :type "CommandPoint Structure"))
  (bind (_location _type _owneractor) (break `CommandPoint` CommandPoint))
  (bind _asbp_squad_player_controller (cast `/Game/AI_Portfolio_Migration/BP_SquadPlayerController` (`GameplayStatics.GetPlayerController` 0)))
  (bind _returnvalue (`SquadPlayerController.GetAvailableMember` _asbp_squad_player_controller (make `CommandPoint` (`SceneComponent.K2_GetComponentLocation` (`self.BombLocation`)) _type _owneractor)))
  (set `self.AssignedSquadMember1` _returnvalue)
  (bind _returnvalue_2 (`SquadPlayerController.GetAvailableMember` _asbp_squad_player_controller (make `CommandPoint` (`SceneComponent.K2_GetComponentLocation` (`self.Assist1`)) _type _owneractor)))
  (set `self.AssignedSquadMember2` _returnvalue_2)
  (bind _returnvalue_3 (`SquadPlayerController.GetAvailableMember` _asbp_squad_player_controller (make `CommandPoint` (`SceneComponent.K2_GetComponentLocation` (`self.Assist2`)) _type _owneractor)))
  (set `self.AssignedSquadMember3` _returnvalue_3))

(fn `OpenDoor`
  (`SceneComponent.K2_AddLocalOffset` (`self.Door`) (0.0 0.0 0.0) false false))

(fn `UserConstructionScript`)