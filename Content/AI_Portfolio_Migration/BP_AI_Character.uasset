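; AI-controlled shooter character that senses incoming fire and takes damage from other AI characters' projectiles, storing its state in the Blackboard.
; BulletDetection overlaps record the shooter as DangerousActor.
; Actor overlaps subtract fixed Health, then test it minus another hit to set IsDead, unpossess and destroy.
; Logic to turn toward the controller's target is present but unconnected.
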(event `self.BulletDetection.OnComponentBeginOverlap`
  (params (OverlappedComponent :type "PrimitiveComponent Object Reference") (OtherActor :type "Actor Object Reference") (OtherComp :type "PrimitiveComponent Object Reference") (OtherBodyIndex :type Integer) (bFromSweep :type Boolean) (SweepResult :type "HitResult Structure (by ref)"))
  (`self.CheckIfInDanger` OtherActor))

(event `self.ReceiveActorBeginOverlap`
  (params (OtherActor :type "Actor Object Reference"))
  (bind _asbp_projectile (cast `/Game/AI_Portfolio_Migration/BP_Projectile` OtherActor))
  (`self.ReduceHealth` _asbp_projectile))

(event `self.ReceiveTick`
  (params (DeltaSeconds :type "Float (single-precision)")))

(fn `CheckIfInDanger`
  (params (Object :type "Object Object Reference"))
  (bind _asbp_projectile (cast `/Game/AI_Portfolio_Migration/BP_Projectile` Object)
    (:`then`
      (bind _shooter (`/Game/AI_Portfolio_Migration/BP_Projectile.Shooter` _asbp_projectile))
      (bind _asbp_ai_character (cast `/Game/AI_Portfolio_Migration/BP_AI_Character` _shooter)
        (:`then`
          (if (!= self _shooter)
            (`BlackboardComponent.SetValueAsObject` (`AIBlueprintHelperLibrary.GetBlackboard` self) "DangerousActor" _asbp_ai_character)
            (return)))
        (:`CastFailed`
          (`VisualLoggerKismetLibrary.LogText` null "Failed cast!" "ShooterObjectName"))))
    (:`CastFailed`
      (`VisualLoggerKismetLibrary.LogText` null "Not Projectile!" "BulletDetection")
      (return))))

(fn `ReduceHealth`
  (params (TheBullet :type "Actor Object Reference"))
  (bind _returnvalue (`AIBlueprintHelperLibrary.GetBlackboard` self))
  (bind _returnvalue_2 (- (`BlackboardComponent.GetValueAsFloat` (`AIBlueprintHelperLibrary.GetBlackboard` self) "Health") 10.0))
  (bind _asbp_projectile (cast `/Game/AI_Portfolio_Migration/BP_Projectile` TheBullet))
  (bind _asbp_ai_character (cast `/Game/AI_Portfolio_Migration/BP_AI_Character` (`/Game/AI_Portfolio_Migration/BP_Projectile.Shooter` _asbp_projectile)))
  (if (not (`KismetStringLibrary.EqualEqual_StrStr` (`KismetSystemLibrary.GetDisplayName` self) (`KismetSystemLibrary.GetDisplayName` _asbp_ai_character)))
    (`BlackboardComponent.SetValueAsFloat` _returnvalue "Health" _returnvalue_2)
    (if (<= _returnvalue_2 0.0)
      (`BlackboardComponent.SetValueAsBool` _returnvalue "IsDead" true)
      (`Controller.UnPossess` (`self.GetController` self))
      (`self.K2_DestroyActor`)
      (return))))

(fn `UserConstructionScript`)