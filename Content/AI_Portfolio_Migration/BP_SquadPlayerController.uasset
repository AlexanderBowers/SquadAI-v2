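; Squad player controller Blueprint that fires projectiles for the controlled first-person character and assigns AI squad members to squad locations.
; FireBPProjectile spawns a BP_Projectile at the character's RealMuzzle, aligns it to the muzzle and launches it along its local forward axis.
; ResetAssignedMember scans all BP_SquadLocation actors and pairs unoccupied ones with squad AI controllers not yet following.
; Each pairing sets the AI's blackboard position and follow flag, then records the member on the location.
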(event `SquadInterface.FireBPProjectile`
  (bind _asbp_squad_first_person_character (cast `/Game/FirstPersonCPP/Blueprints/BP_SquadFirstPersonCharacter` (`self.K2_GetPawn`)))
  (bind _realmuzzle (`/Game/FirstPersonCPP/Blueprints/BP_SquadFirstPersonCharacter.RealMuzzle` _asbp_squad_first_person_character))
  (bind _returnvalue (`|SpawnActorFromClass` "/Game/AI_Portfolio_Migration/BP_Projectile.BP_Projectile_C" (`KismetMathLibrary.Conv_VectorToTransform` (`SceneComponent.K2_GetComponentLocation` _realmuzzle)) "Undefined" "OverrideRootScale" self null))
  (`self.K2_SetActorRotation` _returnvalue (`SceneComponent.K2_GetComponentRotation` _realmuzzle) false)
  (`ProjectileMovementComponent.SetVelocityInLocalSpace` (`/Game/AI_Portfolio_Migration/BP_Projectile.ProjectileMovement` _returnvalue) (1000.0 0.0 0.0)))

(event `SquadInterface.ResetAssignedMember`
  (bind _outactors (`GameplayStatics.GetAllActorsOfClass` "/Game/BP_SquadLocation.BP_SquadLocation_C"))
  (for _array_element _outactors
    (bind _asbp_squad_location (cast `/Game/BP_SquadLocation` _array_element))
    (`KismetSystemLibrary.PrintText` (`KismetTextLibrary.Conv_StringToText` (`KismetSystemLibrary.GetDisplayName` _asbp_squad_location)))
    (`/Engine/EditorBlueprintResources/StandardMacros.IsValid` (`/Game/BP_SquadLocation.AssignedSquadMember` _asbp_squad_location)
      (:`Is Not Valid`
        (for _array_element_2 (`self.SquadMembers`)
          (`/Engine/EditorBlueprintResources/StandardMacros.IsValid` (`/Game/BP_SquadLocation.AssignedSquadMember` _asbp_squad_location)
            (:`Is Not Valid`
              (bind _assquad_aicontroller (cast `SquadAIController` _array_element_2))
              (bind _returnvalue (`AIBlueprintHelperLibrary.GetBlackboard` _assquad_aicontroller))
              (if (not (`BlackboardComponent.GetValueAsBool` _returnvalue "bShouldFollow"))
                (`BlackboardComponent.SetValueAsObject` _returnvalue "AssignedPosition" _array_element)
                (`BlackboardComponent.SetValueAsBool` _returnvalue "bShouldFollow" true)
                (bind _asbp_squad_aicontroller (cast `/Game/AI_Portfolio_Migration/BP_SquadAIController` _assquad_aicontroller))
                (set `/Game/BP_SquadLocation.AssignedSquadMember` _asbp_squad_aicontroller _asbp_squad_location)))))))))

(fn `UserConstructionScript`)